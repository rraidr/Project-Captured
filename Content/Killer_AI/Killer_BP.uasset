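; Killer AI Blueprint with a sight handler that tracks the player through Blackboard keys.
; HandleSightSense ignores non-sight stimuli and actors other than the player character.
; It sets TargetActor to the player while sensed, and on losing sight clears it and saves the stimulus position as LastKnownLocation.
; The event graph is empty, and nothing shown here calls the handler.
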(event EventBeginPlay)

(event Collision|EventActorBeginOverlap
  (params (OtherActor :type Actor%20Object%20Reference)))

(event EventTick
  (params (DeltaSeconds :type Float%20%28single-precision%29)))

(fn ConstructionScript)

(fn HandleSightSense
  (params (Actor :type Actor%20Object%20Reference) (Stimulus :type AI%20Stimulus%20Structure))
  (bind _returnvalue (Class|AIPerceptionSystem|GetSenseClassforStimulus Stimulus))
  (if (== _returnvalue "/Script/AIModule.AISenseConfig_Sight")
    (if (== Actor (Game|GetPlayerCharacter 0))
      (AI|Components|Blackboard|SetValueasObject (AI|GetBlackboard 0) (Utilities|Name|MakeLiteralName "TargetActor") (Utilities|SelectObject (Game|GetPlayerCharacter 0) 0 (.bsuccessfullysensed Stimulus)))
      (if (not (.bsuccessfullysensed Stimulus))
        (AI|Components|Blackboard|SetValueasVector (AI|GetBlackboard 0) (Utilities|Name|MakeLiteralName "LastKnownLocation") (.stimuluslocation Stimulus)))
      (else
        (return)))
    (else
      (return))))
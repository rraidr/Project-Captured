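; Game mode that manages the player's death and respawn cycle and assigns randomized main and secondary stats.
; StatGenerator runs at BeginPlay and after each death, removing the chosen main stat from its pool, while secondary stats can repeat.
; Tick polls the player's Dead flag, counting deaths, triggering spawn-point placement and rerolling stats until the death limit is reached, when the next death opens TestRealm3.
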(event EventBeginPlay
  (bind _asbp_player_character (Utilities|Casting|CastToBP_PlayerCharacter (Game|GetPlayerCharacter 0)))
  (Variables|Default|SetAs%20BP%20Player%20Character _asbp_player_character)
  (CallFunction|StatGenerator))

(event EventTick
  (params (DeltaSeconds :type Float%20%28single-precision%29))
  (bind _as_bp_player_character (Variables|Default|GetAs%20BP%20Player%20Character))
  (if (Variables|/Game/Characters/Player/BP_PlayerCharacter.BP_PlayerCharacter_C|GetDead? _as_bp_player_character)
    (if (< (Variables|Default|GetDeath%20Tracker) 6)
      (bind _result (Math|Integer|IncrementInt (Variables|Default|GetDeath%20Tracker))
        (:%20%20
          (Variables|Default|SetDeath%20Tracker _result)
          (Default|CallSetPlayerSpawnPoint)
          (CallFunction|StatGenerator)
          (Variables|/Game/Characters/Player/BP_PlayerCharacter.BP_PlayerCharacter_C|SetDead? _as_bp_player_character false)))
      (else
        (Game|OpenLevel(byObjectReference) "/Game/Levels/TestRealm3.TestRealm3")))))

(fn ConstructionScript)

(fn StatGenerator
  (bind _mainstat (Variables|Default|GetMainStat))
  (bind _mainstat_2 (Variables|Default|GetMainStat))
  (if (Variables|/Game/Characters/Player/BP_PlayerCharacter.BP_PlayerCharacter_C|GetDead? (Variables|Default|GetAs%20BP%20Player%20Character))
    (bind _output_get (Variables|Default|SetMainStatChoice (.OutItem (Utilities|Array|Random _mainstat_2))))
    (bind _returnvalue (Utilities|Array|RemoveItem _mainstat_2 _output_get))
    (if _returnvalue
      (bind _output_get_2 (Variables|/Game/Characters/Player/BP_PlayerCharacter.BP_PlayerCharacter_C|SetStatDetermination (Variables|Default|GetAs%20BP%20Player%20Character) _output_get))
      (Development|PrintString "First Stat")
      (Development|PrintString (Utilities|String|ToString(Integer) _output_get_2))
      (bind _output_get_3 (Variables|/Game/Characters/Player/BP_PlayerCharacter.BP_PlayerCharacter_C|SetSecondaryStatDetermination (Variables|Default|GetAs%20BP%20Player%20Character) (.OutItem (Utilities|Array|Random (Variables|Default|GetSecondaryStat)))))
      (Development|PrintString "Secondary Stat")
      (Development|PrintString (Utilities|String|ToString(Integer) _output_get_3)))
    (else
      (Utilities|FlowControl|DoOnce false
        (:Completed
          (bind _output_get_4 (Variables|Default|SetMainStatChoice (.OutItem (Utilities|Array|Random _mainstat))))
          (bind _returnvalue_2 (Utilities|Array|RemoveItem _mainstat _output_get_4))
          (if _returnvalue_2
            (bind _output_get_5 (Variables|/Game/Characters/Player/BP_PlayerCharacter.BP_PlayerCharacter_C|SetStatDetermination (Variables|Default|GetAs%20BP%20Player%20Character) _output_get_4))
            (Development|PrintString "First Stat")
            (Development|PrintString (Utilities|String|ToString(Integer) _output_get_5))
            (bind _output_get_6 (Variables|/Game/Characters/Player/BP_PlayerCharacter.BP_PlayerCharacter_C|SetSecondaryStatDetermination (Variables|Default|GetAs%20BP%20Player%20Character) (.OutItem (Utilities|Array|Random (Variables|Default|GetSecondaryStat)))))
            (Development|PrintString "Secondary Stat")
            (Development|PrintString (Utilities|String|ToString(Integer) _output_get_6))))))))
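; BP_TestCrawlSpace is a test crawl space actor that lets the player character enter a small space by crawling.
; On BeginPlay it caches BP_PlayerCharacter and binds its Crawl event through AssignInteract; that event sets EnteringSmallSpace and calls the character's Crawl.
; Two box triggers toggle text renders with opposite logic: Box shows its text while the player overlaps, Box1 hides its own.
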(event OnComponentBeginOverlap(Box)
  (params (OverlappedComponent :type Primitive%20Component%20Object%20Reference) (OtherActor :type Actor%20Object%20Reference) (OtherComp :type Primitive%20Component%20Object%20Reference) (OtherBodyIndex :type Integer) (bFromSweep :type Boolean) (SweepResult :type Hit%20Result%20Structure%20%28by%20ref%29))
  ;[1 1 1] Box 1
  (Utilities|Casting|CastToBP_PlayerCharacter OtherActor)
  (Development|SetHiddeninGame (Variables|Default|GetTextRender) false false))

(event OnComponentEndOverlap(Box)
  (params (OverlappedComponent :type Primitive%20Component%20Object%20Reference) (OtherActor :type Actor%20Object%20Reference) (OtherComp :type Primitive%20Component%20Object%20Reference) (OtherBodyIndex :type Integer))
  ;[1 1 1] Box 1
  (Utilities|Casting|CastToBP_PlayerCharacter OtherActor)
  (Development|SetHiddeninGame (Variables|Default|GetTextRender) true false))

(event OnComponentBeginOverlap(Box1)
  (params (OverlappedComponent :type Primitive%20Component%20Object%20Reference) (OtherActor :type Actor%20Object%20Reference) (OtherComp :type Primitive%20Component%20Object%20Reference) (OtherBodyIndex :type Integer) (bFromSweep :type Boolean) (SweepResult :type Hit%20Result%20Structure%20%28by%20ref%29))
  ;[1 1 1] Box2
  (Utilities|Casting|CastToBP_PlayerCharacter OtherActor)
  (Development|SetHiddeninGame (Variables|Default|GetTextRender1) true false))

(event OnComponentEndOverlap(Box1)
  (params (OverlappedComponent :type Primitive%20Component%20Object%20Reference) (OtherActor :type Actor%20Object%20Reference) (OtherComp :type Primitive%20Component%20Object%20Reference) (OtherBodyIndex :type Integer))
  ;[1 1 1] Box2
  (Utilities|Casting|CastToBP_PlayerCharacter OtherActor)
  (Development|SetHiddeninGame (Variables|Default|GetTextRender1) false false))

(event Custom|Crawl
  (bind _as_bp_player_character (Variables|Default|GetAs%20BP%20Player%20Character))
  (Variables|/Game/Characters/Player/BP_PlayerCharacter.BP_PlayerCharacter_C|SetEnteringSmallSpace _as_bp_player_character true)
  (Default|Crawl _as_bp_player_character))

(event EventBeginPlay
  (bind _asbp_player_character (Utilities|Casting|CastToBP_PlayerCharacter (Game|GetPlayerCharacter 0)))
  (bind _output_get (Variables|Default|SetAs%20BP%20Player%20Character _asbp_player_character))
  (EventDispatchers|AssignInteract _output_get (delegate Custom|Crawl)))

(event Collision|EventActorBeginOverlap
  (params (OtherActor :type Actor%20Object%20Reference)))

(event EventTick
  (params (DeltaSeconds :type Float%20%28single-precision%29)))

(fn ConstructionScript)
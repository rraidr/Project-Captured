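; Test spawn point actor that moves the player to its transform when its ID matches the game mode's death tracker.
; On BeginPlay it caches its root transform and binds SetPlayerSpawn to a PCGameMode event.
; When that event fires and SpawnID equals DeathTracker, it stores the transform as the player character's PlayerSpawnPoint and teleports the capsule there.
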(event Custom|SetPlayerSpawn
  (if (== (Variables|Default|GetSpawnID) (Variables|/Game/Blueprints/Gamemode/PCGameMode.PCGameMode_C|GetDeath%20Tracker (Variables|Default|GetAs%20PCGame%20Mode)))
    (bind _asbp_player_character (Utilities|Casting|CastToBP_PlayerCharacter (Game|GetPlayerCharacter 0)))
    (bind _output_get (Variables|/Game/Characters/Player/BP_PlayerCharacter.BP_PlayerCharacter_C|SetPlayerSpawnPoint _asbp_player_character (Variables|Default|GetSpawn%20Point)))
    (Transformation|SetWorldTransform (Variables|/Script/Engine.Character|GetCapsuleComponent _asbp_player_character) _output_get false true)))

(event EventBeginPlay
  (Variables|Default|SetSpawn%20Point (Transformation|GetWorldTransform (Variables|Default|GetDefaultSceneRoot)))
  (bind _aspcgame_mode (Utilities|Casting|CastToPCGameMode (Game|GetGameMode)))
  (bind _output_get (Variables|Default|SetAs%20PCGame%20Mode _aspcgame_mode))
  (EventDispatchers|BindEventtoSetPlayerSpawnPoint _output_get (delegate Custom|SetPlayerSpawn)))

(event Collision|EventActorBeginOverlap
  (params (OtherActor :type Actor%20Object%20Reference)))

(event EventTick
  (params (DeltaSeconds :type Float%20%28single-precision%29)))

(fn ConstructionScript)
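; Minimal AI character for the crawling system that constantly moves forward, either walking or through CrawlingMovement.
; Crawling status changes switch CharacterMovement between Walking and the custom crawling mode, which Tick checks to choose how to advance.
; Route start and exit events teleport the actor to the door location without a transition, then notify the component it is aligned.
; Query functions report hand IK, permit cover, refuse turning and always request forward movement.
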(event EventMovetoRouteStart
  (params (Route :type CS%20Route%20Actor%20Object%20Reference) (DoorToEnter :type CS_Door%20Enum :default "NewEnumerator0"))
  ;[0 1 0.7882] Minimal setup for entering/exiting routes. Tip: Make a nice transition, like the example in the Firt Person character
  (bind _result (Default|GetEntranceLocation Route DoorToEnter))
  (Transformation|SetActorLocation _result false false)
  (Default|ActorAlignedtoDoorCallback (Variables|Default|GetCrawlingMovement)))

(event EventMovetoRouteExit
  (params (RouteActor :type CS%20Route%20Actor%20Object%20Reference) (DoorToExit :type CS_Door%20Enum :default "NewEnumerator0"))
  ;[0 1 0.7882] Minimal setup for entering/exiting routes. Tip: Make a nice transition, like the example in the Firt Person character
  (bind _result (Default|GetExitLocation RouteActor DoorToExit))
  (Transformation|SetActorLocation _result false false)
  (Default|ActorAlignedtoDoorCallback (Variables|Default|GetCrawlingMovement)))

(event EventBeginPlay
  ;[0 1 0.7882] Minimal setup for handling status changes
  (EventDispatchers|BindEventtoUpdateStatus (Variables|Default|GetCrawlingMovement) (EventDispatchers|CreateEvent :!event CSAICharacterAutoGenFunc)))

(event EventTick
  (params (DeltaSeconds :type Float%20%28single-precision%29))
  (bind _charactermovement (Variables|Character|GetCharacterMovement))
  (if (Pawn|Components|CharacterMovement|IsWalking _charactermovement)
    ;[0 0 0] Default pawn behaviour to make It move foward
    (Pawn|Input|AddMovementInput (Transformation|GetActorForwardVector) 1.0 false)
    (else
      ;[0 1 0.7882] Specific Crawling Movement behaviour to move forward without stopping
      (if (== (Variables|/Script/Engine.CharacterMovementComponent|GetCustomMovementMode _charactermovement) 0)
        (Default|MoveForward (Variables|Default|GetCrawlingMovement))))))

(fn ConstructionScript
  (Default|SetDriverSkeletalMesh (Variables|Default|GetCrawlingMovement) (Variables|Character|GetMesh)))

(fn CSAICharacterAutoGenFunc
  (params (OldStatus :type CS_PlayerStatus%20Enum :default "NewEnumerator0") (NewStatus :type CS_PlayerStatus%20Enum :default "NewEnumerator0"))
  (switch Utilities|FlowControl|Switch|SwitchonCS_PlayerStatus NewStatus ; Enable the new effects
    (:NewEnumerator0
      (Pawn|Components|CharacterMovement|SetMovementMode (Variables|Default|GetCharacterMovement) "MOVE_Walking" 0))
    (:NewEnumerator4
      (Pawn|Components|CharacterMovement|SetMovementMode (Variables|Default|GetCharacterMovement) "MOVE_Custom" (Variables|Default|GetCrawlingCustomChannel)))
    (:NewEnumerator5
      (Pawn|Components|CharacterMovement|SetMovementMode (Variables|Default|GetCharacterMovement) "MOVE_Custom" (Variables|Default|GetCrawlingCustomChannel) :!label _label))
    (:NewEnumerator7
      (goto _label))))

(fn CanTakeCover
  (return true))

(fn CanTurn
  (params (CheckingYaw :type Boolean) (AxisValue :type Float%20%28single-precision%29))
  (return false))

(fn GetCrawlingState
  (return true (Default|GetStatus (Variables|Default|GetCrawlingMovement))))

(fn WillingtoMove
  (return true 1.0))
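; Player controller for the crawling system that lets a tester swap between first-person and third-person characters by pressing the 5 key.
; It queries the possessed pawn's crawling state through a message call and prints a warning instead of swapping when inside a route.
; Otherwise it spawns the other character class at the pawn's transform, possesses it and destroys the previous pawn.
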(event Input|KeyboardEvents|5
  (params (Key :type Key%20Structure :default "None"))
  (:Pressed
    ;[1 1 1] Spawn a new Character for testing other perspective
    (bind _output_get (Variables|Default|SetPreviousPawn (Pawn|GetControlledPawn)))
    (bind _state (Class|BPICSPawn|GetCrawlingState(Message) _output_get))
    (if (Utilities|Enum|Equal(Enum) _state "NewEnumerator0")
      (if (== (Utilities|GetClass _output_get) "/Game/CrawlingSystem/Blueprints/CS_FirstPerson_Character.CS_FirstPerson_Character_C")
        (bind _returnvalue (Game|SpawnActorfromClass "/Game/CrawlingSystem/Blueprints/CS_ThirdPerson_Character.CS_ThirdPerson_Character_C" (Transformation|GetActorTransform _output_get) "AlwaysSpawn" 0 0))
        (Pawn|Possess _returnvalue)
        (else
          (bind _returnvalue_2 (Game|SpawnActorfromClass "/Game/CrawlingSystem/Blueprints/CS_FirstPerson_Character.CS_FirstPerson_Character_C" (Transformation|GetActorTransform _output_get) "AlwaysSpawn" 0 0))
          (Pawn|Possess _returnvalue_2)))
      (Actor|DestroyActor (Variables|Default|GetPreviousPawn))
      (else
        (Development|PrintString "WARNING: You can't swap perspective while inside a route!" true true "(R=1.000000,G=0.687076,B=0.000000,A=1.000000)" 5e+01)))))

(fn ConstructionScript)
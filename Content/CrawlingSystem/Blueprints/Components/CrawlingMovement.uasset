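; Pawn component that drives crawling along a route actor's spline, entered and exited through front or back doors.
; It runs a Standing, Entering, Crawling, Exiting state machine, toggling tagged collision and delegating door alignment to the owner via messages and a callback.
; While crawling, Tick moves the ground-snapped pawn along the spline, facing it forward, and exits at route ends.
; Buffered input changes or stops movement only on animation sync markers.
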(event Custom|MoveForward
  ;[0 1 0.8078] Laid Move Forward/Backwards (we use independent key inputs in case you want to use different ones than the normal movement ones)
  (if (Movement|CanMove)
    (Variables|Movement|SetDirectionBuffer 1.0)))

(event Custom|MoveBackwards
  (bind _routeactor (Variables|References|GetRouteActor))
  ;[0 1 0.8078] Laid Move Forward/Backwards (we use independent key inputs in case you want to use different ones than the normal movement ones)
  (if (Movement|CanMove)
    (if (and (Utilities|IsValid _routeactor) (Variables|/Game/CrawlingSystem/Blueprints/CS_RouteActor.CS_RouteActor_C|GetAllowBackwardMovement _routeactor))
      (Variables|Movement|SetDirectionBuffer -1.0))))

(event EventBeginPlay
  ;[0 1 0.8078] Component initialization
  (bind _aspawn (Utilities|Casting|CastToPawn (Components|GetOwner))
    (:then
      (Variables|References|SetOwnerPawn _aspawn))
    (:CastFailed
      (Development|PrintString "ERROR INIT01: The owner actor must be of type Pawn or a child of It" true true "(R=1.000000,G=0.000000,B=0.037429,A=1.000000)" 5e+01))))

(event EventTick
  (params (DeltaSeconds :type Float%20%28single-precision%29))
  ;[0 1 0.7882] Event Tick
  (if (Utilities|Enum|Equal(Enum) (Variables|Movement|GetActorStatus) "NewEnumerator4")
    (Default|CallCrawlingTick self)
    (|Laid_ForwardMovement)))

(fn ReachedEndOfRoute
  (params (Direction :type Float%20%28single-precision%29))
  (bind _facingdirection (Variables|Movement|GetFacingDirection))
  (bind _distance (Variables|Movement|GetDistance))
  (bind _routeactor (Variables|References|GetRouteActor))
  (bind _routeactor_2 (Variables|References|GetRouteActor))
  (bind _distance_2 (Variables|Movement|GetDistance))
  (bind _returnvalue (>= _facingdirection 0.0))
  (bind _route (Variables|/Game/CrawlingSystem/Blueprints/CS_RouteActor.CS_RouteActor_C|GetRoute _routeactor))
  (bind _returnvalue_2 (Spline|GetSplineLength _route))
  (Utilities|ConvertDirtoEnum Direction
    (:Forward
      (if _returnvalue
        (if (<= (- _returnvalue_2 _distance_2) (Math|Float|Clamp(Float) (Variables|/Game/CrawlingSystem/Blueprints/CS_RouteActor.CS_RouteActor_C|GetDistanceToBackdoorForLeaving _routeactor) 0.2 _returnvalue_2))
          (return true "NewEnumerator1")
          (else
            _))
        (elif (<= (- _returnvalue_2 _distance_2) (Variables|/Game/CrawlingSystem/Blueprints/CS_RouteActor.CS_RouteActor_C|GetDistanceToFrontdoorForLeaving _routeactor))
          (return true "NewEnumerator0")
          (else
            _)))
      (return false "NewEnumerator0"))
    (:Backward
      (if _returnvalue
        (if (<= _distance (Variables|/Game/CrawlingSystem/Blueprints/CS_RouteActor.CS_RouteActor_C|GetDistanceToFrontdoorForLeaving _routeactor_2))
          (return true "NewEnumerator0")
          (else
            _))
        (elif (<= _distance (Math|Float|Clamp(Float) (Variables|/Game/CrawlingSystem/Blueprints/CS_RouteActor.CS_RouteActor_C|GetDistanceToBackdoorForLeaving _routeactor_2) 0.2 (Spline|GetSplineLength (Variables|/Game/CrawlingSystem/Blueprints/CS_RouteActor.CS_RouteActor_C|GetRoute _routeactor_2))))
          (return true "NewEnumerator1")
          (else
            _)))
      (return false "NewEnumerator0"))))

(fn SetLayingVelocity
  (params (Value :type Float%20%28single-precision%29))
  (if (!= Value 0.0)
    (Variables|Movement|SetCurrentSpeed Value)
    (else
      (Variables|Movement|SetCurrentSpeed 0.0))))

(fn StopMovementInmediatly
  (Variables|Movement|SetMovementDirection 0.0)
  (Movement|SetLayingVelocity 0.0))

(fn UpdateDistanceAlongSpline
  (params (Increase :type Float%20%28single-precision%29))
  (Variables|Movement|SetDistance (Math|Float|Clamp(Float) (+ (Variables|Movement|GetDistance) Increase) 0.0 (- (Spline|GetSplineLength (Variables|/Game/CrawlingSystem/Blueprints/CS_RouteActor.CS_RouteActor_C|GetRoute (Variables|References|GetRouteActor))) 0.001))))

(fn SetLayingStatus
  (params (NewCrawling :type Boolean))
  (if NewCrawling
    (bind _output_get (LocalVariables|SetPrevStatus (Variables|Movement|GetActorStatus)))
    (bind _output_get_2 (Variables|Movement|SetActorStatus "NewEnumerator4"))
    (Default|CallUpdateStatus _output_get _output_get_2)
    (Variables|Movement|SetMovementDirection 1.0) ; Adds the feeling of entering somwhere. This is optional to move the player a bit forward when entered the route
    (else
      (bind _output_get_3 (LocalVariables|SetPrevStatus (Variables|Movement|GetActorStatus)))
      (bind _output_get_4 (Variables|Movement|SetActorStatus "NewEnumerator0"))
      (Default|CallUpdateStatus _output_get_3 _output_get_4)
      (Controller|SetControllerRotation) ; We need to set the controller rotation to match the exit direction (like the actor rotation does)
    )))

(fn SetControllerRotation
  (bind _ownerpawn (Variables|References|GetOwnerPawn))
  (bind _returnvalue (Transformation|GetActorRotation _ownerpawn))
  (Pawn|SetControlRotation (Pawn|GetController _ownerpawn) (Math|Rotator|MakeRotator (.roll _returnvalue) (.pitch _returnvalue) (.yaw _returnvalue))))

(fn GetRouteStartLocation
  (params (Door :type CS_Door%20Enum :default "NewEnumerator0") (RouteActor :type CS%20Route%20Actor%20Object%20Reference))
  (bind _newparam (Utils|GetZOffset))
  (switch Utilities|FlowControl|Switch|SwitchonCS_Door Door
    (:NewEnumerator0
      (bind _location (Default|GetGroundCollisionLocation RouteActor 0.0))
      (LocalVariables|SetLoc (Math|Vector|MakeVector (.x _location) (.y _location) (+ (.z _location) _newparam))))
    (:NewEnumerator1
      (bind _location_2 (Default|GetGroundCollisionLocation RouteActor (- (Spline|GetSplineLength (Variables|/Game/CrawlingSystem/Blueprints/CS_RouteActor.CS_RouteActor_C|GetRoute RouteActor)) 0.001)))
      (LocalVariables|SetLoc (Math|Vector|MakeVector (.x _location_2) (.y _location_2) (+ (.z _location_2) _newparam)))))
  (return (LocalVariables|GetLoc)))

(fn GetActorDistanceatSpline
  (params (ExtraOffset :type Float%20%28single-precision%29))
  (bind _routeactor (Variables|References|GetRouteActor))
  (bind _distance (Variables|Movement|GetDistance))
  (bind _route (Variables|/Game/CrawlingSystem/Blueprints/CS_RouteActor.CS_RouteActor_C|GetRoute _routeactor))
  (bind _returnvalue (Spline|GetSplineLength _route))
  (if (== (Variables|Movement|GetFacingDirection) 1.0)
    (return (Math|Float|Clamp(Float) (+ _distance ExtraOffset) 0.0 (Spline|GetSplineLength _route)))
    (else
      (return (Math|Float|Clamp(Float) (- _returnvalue (+ _distance ExtraOffset)) 0.0 (- _returnvalue 0.1))))))

(fn ToggleDebugVisuals
  (if (Variables|Options|GetDebug)
    _))

(fn TryTakeCover
  (params (RouteActor :type CS%20Route%20Actor%20Object%20Reference) (Door :type CS_Door%20Enum :default "NewEnumerator0"))
  ;[0 1 0.8078] Check if Pawn Actor can go to crawling state
  (Utilities|IsValid RouteActor
    (:Is%20Valid
      (bind _cando (Class|BPICSPawn|CanTakeCover(Message) (Variables|References|GetOwnerPawn)))
      (if (and _cando (Utilities|Enum|Equal(Enum) (Variables|Movement|GetActorStatus) "NewEnumerator0"))
        (Variables|References|SetRouteActor RouteActor)
        (switch Utilities|FlowControl|Switch|SwitchonCS_Door Door
          (:NewEnumerator0
            (Variables|Movement|SetFacingDirection 1.0))
          (:NewEnumerator1
            (Variables|Movement|SetFacingDirection -1.0)))
        (bind _output_get (LocalVariables|SetPrevStatus (Variables|Movement|GetActorStatus)))
        (bind _output_get_2 (Variables|Movement|SetActorStatus "NewEnumerator5"))
        (Default|CallUpdateStatus _output_get _output_get_2) ; Tell owner actor the status changed
        (Movement|TogglePawnCollision false)
        (Variables|Movement|SetDistance 0.0) ; Reset distance
        (Class|BPICSPawn|MovetoRouteStart(Message) (Variables|References|GetOwnerPawn) RouteActor Door)
        (return true)
        (else
          _)))
    (:Is%20Not%20Valid
      _))
  (return false))

(fn TryLeaveCover
  (params (Door :type CS_Door%20Enum :default "NewEnumerator0"))
  (if (and (Utilities|Enum|Equal(Enum) (Variables|Movement|GetActorStatus) "NewEnumerator4") (Utilities|IsValid (Variables|References|GetRouteActor)))
    (Variables|Movement|SetActorStatus "NewEnumerator7")
    (Movement|TogglePawnCollision true)
    (Variables|Movement|SetDistance 0.0)
    (Class|BPICSPawn|MovetoRouteExit(Message) (Variables|References|GetOwnerPawn) (Variables|References|GetRouteActor) Door)
    (return true)
    (else
      (return false))))

(fn OrientateActorTowardsSpline
  (bind _routeactor (Variables|References|GetRouteActor))
  (bind _ownerpawn (Variables|References|GetOwnerPawn))
  (bind _returnvalue (Transformation|GetActorRotation _ownerpawn))
  (bind _route (Variables|/Game/CrawlingSystem/Blueprints/CS_RouteActor.CS_RouteActor_C|GetRoute _routeactor))
  ;[0 0 0] Orient actor itself
  (Transformation|SetActorRotation _ownerpawn (Math|Rotator|MakeRotator (.roll _returnvalue) (.pitch _returnvalue) (.yaw (Math|Rotator|FindLookatRotation (Spline|GetLocationatDistanceAlongSpline _route (Route|GetActorDistanceatSpline 0.0) "World") (Spline|GetLocationatDistanceAlongSpline _route (Route|GetActorDistanceatSpline 0.5) "World"))))))

(fn SetDriverSkeletalMesh
  (params (DriverSkeleton :type Skeletal%20Mesh%20Component%20Object%20Reference))
  (Variables|Default|SetDriverSkelMesh DriverSkeleton))

(fn TogglePawnCollision
  (params (NewEnabled :type Boolean))
  (for _array_element (Actor|GetComponentsbyTag (Components|GetOwner) "/Script/Engine.ShapeComponent" (Variables|Movement|GetCollisionTag))
    (if NewEnabled
      (Collision|SetCollisionEnabled _array_element "QueryAndPhysics")
      (else
        (Collision|SetCollisionEnabled _array_element "NoCollision")))))

(fn GetZOffset
  ;[0.251 1 0.902] If the owner pawn is of class Character, get capsule half height for calculations, otherwise dont add offset
  (bind _ascharacter (Utilities|Casting|CastToCharacter (Variables|References|GetOwnerPawn))
    (:then
      (return (Components|Capsule|GetScaledCapsuleHalfHeight (Variables|/Script/Engine.Character|GetCapsuleComponent _ascharacter))))
    (:CastFailed
      (return 0.0))))

(fn GetStatus
  (return (Variables|Movement|GetActorStatus)))

(fn GetMovementDirection
  (return (Variables|Movement|GetMovementDirection)))

(fn GetRouteActor
  (return (Variables|References|GetRouteActor)))

(fn ActorAlignedtoDoorCallback
  (switch Utilities|FlowControl|Switch|SwitchonCS_PlayerStatus (Variables|Movement|GetActorStatus)
    (:NewEnumerator5
      (Movement|SetLayingStatus true))
    (:NewEnumerator7
      (Movement|SetLayingStatus false))))

(fn GetMovementSpeed
  (return (Variables|Movement|GetCurrentSpeed)))

(fn CanStopMovement
  (bind _willingtomove (Class|BPICSPawn|WillingtoMove(Message) (Variables|References|GetOwnerPawn)))
  (return (not _willingtomove)))

(fn CanMove
  (return (and (Variables|Options|GetAllowPlayerInput) (Utilities|Enum|Equal(Enum) (Variables|Movement|GetActorStatus) "NewEnumerator4"))))

(fn MoveActorAlongSpline
  (params (Direction :type Float%20%28single-precision%29))
  (bind _speedlaid_forward (Variables|Movement|GetSpeedLaid_Forward))
  (bind _speedlaid_backwards (Variables|Movement|GetSpeedLaid_Backwards))
  (bind _returnvalue (* _speedlaid_backwards -1.0))
  (if (> Direction 0.0)
    (Movement|UpdateDistanceAlongSpline _speedlaid_forward)
    (Movement|SetLayingVelocity _speedlaid_forward)
    (else
      (Movement|UpdateDistanceAlongSpline _returnvalue)
      (Movement|SetLayingVelocity _returnvalue)))
  ;[0.4129 1 0.04518] Forward movement
  (bind _location (Default|GetGroundCollisionLocation (Variables|References|GetRouteActor) (Route|GetActorDistanceatSpline 0.0)))
  (Transformation|SetActorLocation (Variables|References|GetOwnerPawn) (Math|Vector|MakeVector (.x _location) (.y _location) (+ (.z _location) (Utils|GetZOffset))) false false)
  (Movement|OrientateActorTowardsSpline))

(fn ShouldLeaveCover
  (bind (_routeend _exitdoor) (Route|ReachedEndOfRoute (Variables|Movement|GetMovementDirection)))
  (bind _willingtomove (Class|BPICSPawn|WillingtoMove(Message) (Variables|References|GetOwnerPawn)))
  (return _exitdoor (and _willingtomove _routeend)))

(fn GetActorStatus
  (return (Variables|Movement|GetActorStatus)))

(fn CatchAnimMarker
  (return (Class|AnimInstance|HasMarkerBeenHitThisFrame (Components|SkeletalMesh|GetAnimInstance (Variables|Default|GetDriverSkelMesh)) (Variables|Animation|GetAnimSyncGroup) (Variables|Animation|GetAnimMarkerName))))
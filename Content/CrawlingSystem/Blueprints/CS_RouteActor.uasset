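; Spline-based crawl route with a front and back door for entering and leaving.
; While the route is enabled, door triggers call TryTakeCover on an overlapping actor's CrawlingMovement component, passing the route and door.
; The construction script positions the back trigger, exit points and exit-limit markers from the spline, applies debug visibility, and enables back-door overlaps only for bidirectional routes.
; Helpers provide exit locations and ground-traced entrance locations.
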(event OnComponentBeginOverlap(BackDoorTrigger)
  (params (OverlappedComponent :type Primitive%20Component%20Object%20Reference) (OtherActor :type Actor%20Object%20Reference) (OtherComp :type Primitive%20Component%20Object%20Reference) (OtherBodyIndex :type Integer) (bFromSweep :type Boolean) (SweepResult :type Hit%20Result%20Structure%20%28by%20ref%29))
  (bind _returnvalue (Actor|GetComponentbyClass OtherActor "/Game/CrawlingSystem/Blueprints/Components/CrawlingMovement.CrawlingMovement_C"))
  (if (Variables|CrawlSystemConfig|GetRouteEnabled)
    (Utilities|IsValid _returnvalue
      (:Is%20Valid
        (Default|TryTakeCover _returnvalue self "NewEnumerator1")))))

(event OnComponentBeginOverlap(FrontDoorTrigger)
  (params (OverlappedComponent :type Primitive%20Component%20Object%20Reference) (OtherActor :type Actor%20Object%20Reference) (OtherComp :type Primitive%20Component%20Object%20Reference) (OtherBodyIndex :type Integer) (bFromSweep :type Boolean) (SweepResult :type Hit%20Result%20Structure%20%28by%20ref%29))
  (bind _returnvalue (Actor|GetComponentbyClass OtherActor "/Game/CrawlingSystem/Blueprints/Components/CrawlingMovement.CrawlingMovement_C"))
  (if (Variables|CrawlSystemConfig|GetRouteEnabled)
    (Utilities|IsValid _returnvalue
      (:Is%20Valid
        (Default|TryTakeCover _returnvalue self "NewEnumerator0")))))

(fn ConstructionScript
  (Utilities|FlowControl|Sequence
    (:then_0
      (Functional|Location|PlaceBackdoorTrigger))
    (:then_1
      (Functional|Location|PlaceExitLocationPoints))
    (:then_2
      (Debug|PlaceExitLimitsVisuals))
    (:then_3
      (Debug|ShowDebugVisuals (Variables|CrawlSystemConfig|GetDebug)))
    (:then_4
      (Functional|ToggleBackdoorTrigger (Variables|CrawlSystemConfig|GetBiDirectionalRoute)))))

(fn DrawGroundCollisionDebug
  (bind _route (Variables|Default|GetRoute))
  (bind _returnvalue (Spline|GetSplineLength _route))
  (while (<= (LocalVariables|GetDistance) _returnvalue)
    (Collision|LineTraceByChannel (Spline|GetLocationatDistanceAlongSpline _route (Math|Float|%(Float) (LocalVariables|GetDistance) _returnvalue) "World") (+ (Spline|GetLocationatDistanceAlongSpline _route (Math|Float|%(Float) (LocalVariables|GetDistance) _returnvalue) "World") (* (Class|SplineComponent|GetUpVectoratDistanceAlongSpline _route (Math|Float|%(Float) (LocalVariables|GetDistance) _returnvalue) "World") -1e+02)) "TraceTypeQuery1" false 0 "ForDuration" false "(R=1.000000,G=0.000000,B=0.000000,A=1.000000)" "(R=0.000000,G=1.000000,B=0.000000,A=1.000000)" 6e+01)
    (LocalVariables|SetDistance (+ (LocalVariables|GetDistance) 1.0))))

(fn GetGroundCollisionLocation
  (params (Distance :type Float%20%28single-precision%29))
  (bind _route (Variables|Default|GetRoute))
  (bind _returnvalue (Spline|GetSplineLength _route))
  (bind _returnvalue_2 (Math|Float|%(Float) Distance _returnvalue))
  (bind _returnvalue_3 (Spline|GetLocationatDistanceAlongSpline _route _returnvalue_2 "World"))
  (bind (_outhit _returnvalue_4) (Collision|LineTraceByChannel _returnvalue_3 (+ _returnvalue_3 (* (Class|SplineComponent|GetUpVectoratDistanceAlongSpline _route _returnvalue_2 "World") -1e+02)) "TraceTypeQuery1" false 0 "None" false "(R=1.000000,G=0.000000,B=0.000000,A=1.000000)" "(R=0.000000,G=1.000000,B=0.000000,A=1.000000)" 1e+03))
  (return (.Location (Collision|BreakHitResult _outhit)) _outhit _returnvalue_4))

(fn GetExitLocation
  (params (ExitDoor :type CS_Door%20Enum :default "NewEnumerator0"))
  (switch Utilities|FlowControl|Switch|SwitchonCS_Door ExitDoor
    (:NewEnumerator0
      (LocalVariables|SetLoc (Transformation|GetWorldLocation (Variables|Default|GetFrontDoor_ExitPoint))))
    (:NewEnumerator1
      (LocalVariables|SetLoc (Transformation|GetWorldLocation (Variables|Default|GetBackDoor_ExitPoint)))))
  (return (LocalVariables|GetLoc)))

(fn ShowDebugVisuals
  (params (Debug :type Boolean))
  (bind _frontdoortrigger (Variables|Default|GetFrontDoorTrigger))
  (bind _output_get (Variables|CrawlSystemConfig|SetDebug Debug))
  (if _output_get
    (if (Variables|CrawlSystemConfig|GetBiDirectionalRoute)
      (Development|SetHiddeninGame _frontdoortrigger false true)
      (else
        (Development|SetHiddeninGame _frontdoortrigger false true)))
    (else
      (Development|SetHiddeninGame _frontdoortrigger true true))))

(fn SetDebugging
  (params (Debug :type Boolean))
  (Debug|ShowDebugVisuals Debug))

(fn PlaceExitLimitsVisuals
  (bind _route (Variables|Default|GetRoute))
  (bind _distancetofrontdoorforleaving (Variables|CrawlSystemConfig|GetDistanceToFrontdoorForLeaving))
  (bind _distancetobackdoorforleaving (Variables|CrawlSystemConfig|GetDistanceToBackdoorForLeaving))
  (bind _returnvalue (Spline|GetSplineLength _route))
  (bind _returnvalue_2 (- _returnvalue _distancetobackdoorforleaving))
  (Transformation|SetWorldLocationAndRotation (Variables|Default|GetFrontDoor_exitlimit) (Spline|GetLocationatDistanceAlongSpline _route _distancetofrontdoorforleaving "World") (Spline|GetRotationatDistanceAlongSpline _route _distancetofrontdoorforleaving "World") false false)
  (Transformation|SetWorldLocationAndRotation (Variables|Default|GetBackDoor_exitlimit) (Spline|GetLocationatDistanceAlongSpline _route _returnvalue_2 "World") (Spline|GetRotationatDistanceAlongSpline _route _returnvalue_2 "World") false false))

(fn PlaceExitLocationPoints
  (bind _frontdoor_exitpoint (Variables|Default|GetFrontDoor_ExitPoint))
  (bind _backdoor_exitpoint (Variables|Default|GetBackDoor_ExitPoint))
  (bind _backdoor_exitlocationdistance (Variables|CrawlSystemConfig|GetBackdoor_ExitLocationDistance))
  (bind _frontdoor_exitlocationdistance (Variables|CrawlSystemConfig|GetFrontdoor_ExitLocationDistance))
  (bind _route (Variables|Default|GetRoute))
  (bind _returnvalue (Spline|GetLocationatSplinePoint _route 0 "Local"))
  (bind _returnvalue_2 (Class|SplineComponent|GetDirectionatSplinePoint _route 0 "Local"))
  (bind _returnvalue_3 (Spline|GetNumberOfSplinePoints _route))
  (bind _returnvalue_4 (* _frontdoor_exitlocationdistance -1.0))
  (bind _returnvalue_5 (* _returnvalue_2 _returnvalue_4))
  (bind _returnvalue_6 (- _returnvalue_3 1))
  (bind _returnvalue_7 (Class|SplineComponent|GetDirectionatSplinePoint _route _returnvalue_6 "Local"))
  (bind _returnvalue_8 (Spline|GetLocationatSplinePoint _route _returnvalue_6 "Local"))
  (bind _returnvalue_9 (+ _returnvalue_5 _returnvalue))
  (bind _returnvalue_10 (* _returnvalue_7 _backdoor_exitlocationdistance))
  (bind _returnvalue_11 (+ _returnvalue_10 _returnvalue_8))
  (Transformation|SetRelativeLocation _backdoor_exitpoint (Math|Conversions|ToVector(Vector2D) (Math|Vector2D|MakeVector2D (.x _returnvalue_11) (.y _returnvalue_11)) (+ (.z _returnvalue_11) (.z (Variables|/Script/Engine.SceneComponent|GetRelativeLocation _backdoor_exitpoint)))) false false)
  (Transformation|SetRelativeLocation _frontdoor_exitpoint (Math|Conversions|ToVector(Vector2D) (Math|Vector2D|MakeVector2D (.x _returnvalue_9) (.y _returnvalue_9)) (+ (.z _returnvalue_9) (.z (Variables|/Script/Engine.SceneComponent|GetRelativeLocation _frontdoor_exitpoint)))) false false))

(fn PlaceBackdoorTrigger
  (bind _route (Variables|Default|GetRoute))
  (Transformation|SetWorldLocation (Variables|Default|GetBackDoorTrigger) (Spline|GetLocationatSplinePoint _route (- (Spline|GetNumberOfSplinePoints _route) 1) "World") false false))

(fn ToggleBackdoorTrigger
  (params (Enabled :type Boolean))
  (Variables|/Script/Engine.PrimitiveComponent|SetbGenerateOverlapEvents (Variables|Default|GetBackDoorTrigger) Enabled))

(fn GetEntranceLocation
  (params (EntrancetDoor :type CS_Door%20Enum :default "NewEnumerator0"))
  (switch Utilities|FlowControl|Switch|SwitchonCS_Door EntrancetDoor
    (:NewEnumerator0
      (bind _location (Functional|Location|GetGroundCollisionLocation 0.0))
      (LocalVariables|SetLoc _location))
    (:NewEnumerator1
      (bind _location_2 (Functional|Location|GetGroundCollisionLocation (- (Spline|GetSplineLength (Variables|Default|GetRoute)) 0.001)))
      (LocalVariables|SetLoc _location_2)))
  (return (LocalVariables|GetLoc)))